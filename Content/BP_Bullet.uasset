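; Paper2D bullet locked to Y=0 that travels in one of eight string-coded directions and bounces off rebound walls.
; Shoot starts a fast looping timer that moves it along its Arrow and counts down its lifetime, while Tick rotates the flipbook to match the direction.
; Overlaps destroy it, except rebound walls, whose facing remaps the direction through a lookup.
; Dash halts the countdown and drives speed by timeline, destroying the bullet when finished.
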(event `Shoot`
  (params (BaseDirection :type String))
  (set `self.Direction(String)` BaseDirection)
  (bind _returnvalue (`KismetSystemLibrary.K2_SetTimerDelegate` (delegate `Move(Normal)`) 0.0002 true))
  (set `self.Timer(NormalMove)` _returnvalue))

(event `Move(Normal)`
  (`|ExecutionSequence`
    (:`then_0`
      (`self.K2_AddActorWorldOffset` (* (`SceneComponent.GetForwardVector` (`self.Arrow`)) (`self.MoveSpeed`))))
    (:`then_1`
      (if (not (`self.bIsDash`))
        (bind _output_get (set `self.LifeCycle` (- (`self.LifeCycle`) 0.0002)))
        (if (<= _output_get 0.0)
          (`KismetSystemLibrary.K2_ClearAndInvalidateTimerHandle` (stale `Shoot` _returnvalue))
          (`self.K2_DestroyActor`))))))

(event `self.ReceiveTick`
  (params (DeltaSeconds :type "Float (single-precision)"))
  (`|ExecutionSequence`
    (:`then_0`
      (switch `string` (`self.Direction(String)`)
        (:`L`
          (set `self.RelativeRotation` (struct :`Pitch` 90.0)))
        (:`LU`
          (set `self.RelativeRotation` (struct :`Pitch` 45.0)))
        (:`LD`
          (set `self.RelativeRotation` (struct :`Pitch` -135.0 :`Yaw` 180.0)))
        (:`U`
          (set `self.RelativeRotation` (struct)))
        (:`D`
          (set `self.RelativeRotation` (struct :`Pitch` -180.0)))
        (:`RU`
          (set `self.RelativeRotation` (struct :`Pitch` -45.0)))
        (:`RD`
          (set `self.RelativeRotation` (struct :`Pitch` -135.0)))
        (:`R`
          (set `self.RelativeRotation` (struct :`Pitch` -90.0))))
      (`SceneComponent.K2_SetWorldRotation` (`self.PaperFlipbook`) (`self.RelativeRotation`) false false))))

(event `Dash`
  (set `self.bIsDash` true)
  (bind (_direction _alpha) (`Timeline|Timeline_0` :!via `PlayFromStart`)
    (:`Update`
      (set `self.MoveSpeed` (`KismetMathLibrary.Lerp` 0.5 0.1 _alpha)))
    (:`Finished`
      (`self.K2_DestroyActor`))))

(event `self.ww.OnComponentBeginOverlap`
  (params (OverlappedComponent :type "PrimitiveComponent Object Reference") (OtherActor :type "Actor Object Reference") (OtherComp :type "PrimitiveComponent Object Reference") (OtherBodyIndex :type Integer) (bFromSweep :type Boolean) (SweepResult :type "HitResult Structure (by ref)"))
  (switch `string` (`KismetSystemLibrary.GetClassDisplayName` (`GameplayStatics.GetObjectClass` OtherActor))
    (:`Default`
      (`self.K2_DestroyActor`))
    (:`BP_ReboundWall_C`
      (bind _asbp_rebound_wall (cast `/Game/BP_ReboundWall` OtherActor))
      (`/Engine/EditorBlueprintResources/StandardMacros.IsValid` _asbp_rebound_wall
        (:`Is Valid`
          (switch `string` (`/Game/BP_ReboundWall.BaseDirection` _asbp_rebound_wall)
            (:`L`
              (switch `string` (`self.Direction(String)`)
                (:`RU`
                  (set `self.Direction(String)` "LU"))
                (:`RD`
                  (set `self.Direction(String)` "LD"))
                (:`R`
                  (set `self.Direction(String)` "L"))))
            (:`LU`
              (switch `string` (`self.Direction(String)`)
                (:`R`
                  (set `self.Direction(String)` "U"))
                (:`RD`
                  (set `self.Direction(String)` "LU"))
                (:`D`
                  (set `self.Direction(String)` "L"))))
            (:`LD`
              (switch `string` (`self.Direction(String)`)
                (:`R`
                  (set `self.Direction(String)` "D"))
                (:`RU`
                  (set `self.Direction(String)` "LD"))
                (:`U`
                  (set `self.Direction(String)` "L"))))
            (:`U`
              (switch `string` (`self.Direction(String)`)
                (:`D`
                  (set `self.Direction(String)` "U"))
                (:`LD`
                  (set `self.Direction(String)` "LU"))
                (:`RD`
                  (set `self.Direction(String)` "RU"))))
            (:`D`
              (switch `string` (`self.Direction(String)`)
                (:`U`
                  (set `self.Direction(String)` "D"))
                (:`LU`
                  (set `self.Direction(String)` "LD"))
                (:`RU`
                  (set `self.Direction(String)` "RD"))))
            (:`RU`
              (switch `string` (`self.Direction(String)`)
                (:`D`
                  (set `self.Direction(String)` "R"))
                (:`LD`
                  (set `self.Direction(String)` "RU"))
                (:`L`
                  (set `self.Direction(String)` "U"))))
            (:`RD`
              (switch `string` (`self.Direction(String)`)
                (:`U`
                  (set `self.Direction(String)` "R"))
                (:`LU`
                  (set `self.Direction(String)` "RD"))
                (:`L`
                  (set `self.Direction(String)` "D"))))
            (:`R`
              (switch `string` (`self.Direction(String)`)
                (:`LD`
                  (set `self.Direction(String)` "RD"))
                (:`LU`
                  (set `self.Direction(String)` "RU"))
                (:`L`
                  (set `self.Direction(String)` "R"))))))))))

(fn `UserConstructionScript`
  (bind (_returnvalue_x _returnvalue_y _returnvalue_z) (`KismetMathLibrary.BreakVector` (`self.K2_GetActorLocation`)))
  (`self.K2_SetActorLocation` (`KismetMathLibrary.MakeVector` _returnvalue_x 0.0 _returnvalue_z)))