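; BP_ReboundWall is a Paper2D wall actor that can face one of eight cardinal or diagonal directions.
; Its construction script maps BaseDirection to a preset rotation and applies it to the sprite in world space.
; It also snaps the actor's Y to zero, keeping it on the 2D plane.
; The event graph holds only disabled stubs, so any rebound behavior is not scripted here.
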(fn `UserConstructionScript`
  (bind (_returnvalue_x _returnvalue_y _returnvalue_z) (`KismetMathLibrary.BreakVector` (`self.K2_GetActorLocation`)))
  (`|ExecutionSequence`
    (:`then_0`
      (switch `string` (`self.BaseDirection`)
        (:`L`
          (set `self.RelativeRotation` (struct :`Pitch` 90.0)))
        (:`LU`
          (set `self.RelativeRotation` (struct :`Pitch` 45.0)))
        (:`LD`
          (set `self.RelativeRotation` (struct :`Pitch` -135.0 :`Yaw` 180.0)))
        (:`U`
          (set `self.RelativeRotation` (struct)))
        (:`D`
          (set `self.RelativeRotation` (struct :`Pitch` -180.0)))
        (:`RU`
          (set `self.RelativeRotation` (struct :`Pitch` -45.0)))
        (:`RD`
          (set `self.RelativeRotation` (struct :`Pitch` -135.0)))
        (:`R`
          (set `self.RelativeRotation` (struct :`Pitch` -90.0))))
      (`SceneComponent.K2_SetWorldRotation` (`self.PaperSprite`) (`self.RelativeRotation`) false false))
    (:`then_1`
      (`self.K2_SetActorLocation` (`KismetMathLibrary.MakeVector` _returnvalue_x 0.0 _returnvalue_z)))))